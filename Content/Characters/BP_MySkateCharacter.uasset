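; Skateboarding player character Blueprint that switches its movement component to a custom Skate mode on BeginPlay.
; P plays a push montage and adds a forward velocity impulse, while Space adds an upward "fake ollie" impulse only in Skate mode.
; Tick flips the camera boom 180 degrees whenever velocity opposes the capsule's forward vector.
; An unconnected rotate-to-floor alignment snippet never runs.
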(event `self.ReceiveBeginPlay`
  (`CharacterMovementComponent.SetMovementMode` (`self.CharacterMovement`) "MOVE_Custom" (enumliteral `ECustomMovementMode` "CMOVE_Skate")))

(event `Key|P`
  (params (Key :type "Key Structure"))
  (:`Pressed`
    (`KismetSystemLibrary.PrintString` "PUSH")
    (`|PlayMontage` (`self.Mesh`) "/Game/SkateAssets/Animations/SkatePush_Montage.SkatePush_Montage"
      (:`then`
        (`CharacterMovementComponent.AddImpulse` (`self.CharacterMovement`) (* (`SceneComponent.GetForwardVector` (`self.CapsuleComponent`)) 700.0) true)))))

(event `Key|SpaceBar`
  (params (Key :type "Key Structure"))
  (bind _charactermovement (`self.CharacterMovement`))
  (:`Pressed`
    (bind _asskate_character_movement_component (cast `SkateCharacterMovementComponent` _charactermovement))
    (if (`SkateCharacterMovementComponent.IsCustomMovementMode` _asskate_character_movement_component "CMOVE_Skate")
      (`KismetSystemLibrary.PrintString` "FAKE OLLIE")
      (`CharacterMovementComponent.AddImpulse` _charactermovement (* (`SceneComponent.GetUpVector` (`self.CapsuleComponent`)) 700.0) true))))

(event `self.ReceiveTick`
  (params (DeltaSeconds :type "Float (single-precision)"))
  (if (< (`KismetMathLibrary.Dot_VectorVector` (`SceneComponent.GetForwardVector` (`self.CapsuleComponent`)) (`MovementComponent.Velocity` (`self.CharacterMovement`))) 0.0)
    (`SceneComponent.K2_SetRelativeRotation` (`self.CameraBoom`) (struct :`Yaw` 180.0) false false)
    (else
      (`SceneComponent.K2_SetRelativeRotation` (`self.CameraBoom`) (struct) false false))))

(fn `UserConstructionScript`)