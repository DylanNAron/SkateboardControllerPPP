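; BP_GrindableObstacle is a spline-shaped obstacle that the skate character grinds along.
; Its construction script tiles GrindMesh as instanced static meshes along GrindSpline, spaced by mesh length plus Offset.
; Hitting the mesh disables character movement and starts grinding from the nearest spline point.
; Tick then moves the character atop the spline one unit per frame, with no exit logic and debug prints throughout.
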(event `self.ReceiveBeginPlay`
  (set `self.GrindMeshHeight` (* (.z (`.BoxExtent` (`KismetMathLibrary.BreakBoxSphereBounds` (`StaticMesh.GetBounds` (`self.GrindMesh`))))) 2.0)))

(event `self.InstancedStaticMesh.OnComponentHit`
  (params (HitComponent :type "PrimitiveComponent Object Reference") (OtherActor :type "Actor Object Reference") (OtherComp :type "PrimitiveComponent Object Reference") (NormalImpulse :type "Vector Structure") (Hit :type "HitResult Structure (by ref)"))
  (bind _grindspline (`self.GrindSpline`))
  (bind _asbp_my_skate_character (cast `/Game/Characters/BP_MySkateCharacter` OtherActor))
  (if (not (`self.isGrinding`))
    (bind _output_get (set `self.As BP My Skate Character` _asbp_my_skate_character))
    (set `self.isGrinding` true)
    (set `self.DistanceAlongSpline` (`SplineComponent.GetDistanceAlongSplineAtSplineInputKey` _grindspline (`SplineComponent.FindInputKeyClosestToWorldLocation` _grindspline (`self.K2_GetActorLocation` _asbp_my_skate_character))))
    (`KismetSystemLibrary.PrintString` "ITS GRIND TIME")
    (`CharacterMovementComponent.SetMovementMode` (`Character.CharacterMovement` _output_get) "MOVE_None" 0)))

(event `self.ReceiveTick`
  (params (DeltaSeconds :type "Float (single-precision)"))
  (bind (_returnvalue_x _returnvalue_y _returnvalue_z) (`KismetMathLibrary.BreakVector` (`SplineComponent.GetLocationAtDistanceAlongSpline` (`self.GrindSpline`) (`self.DistanceAlongSpline`) "World")))
  (if (`self.isGrinding`)
    (`self.K2_SetActorLocation` (`self.As BP My Skate Character`) (`KismetMathLibrary.MakeVector` _returnvalue_x _returnvalue_y (+ (`CapsuleComponent.GetScaledCapsuleHalfHeight` (`Character.CapsuleComponent` (`self.As BP My Skate Character`))) (+ _returnvalue_z (`self.GrindMeshHeight`)))) false false)
    (set `self.DistanceAlongSpline` (+ (`self.DistanceAlongSpline`) 1.0))
    (`KismetSystemLibrary.PrintString` "SHREDUT ABD EDUT")))

(fn `GetLocationAtIndex`
  (params (A :type Integer))
  (returns (ReturnValue :type "Vector Structure"))
  (return (`SplineComponent.GetLocationAtDistanceAlongSpline` (`self.GrindSpline`) (* A (`self.Spacing`)) "Local")))

(fn `UserConstructionScript`
  (locals (`Number of Instances` :type Integer :default 0))
  (bind (_min _max) (break `Box` (`StaticMesh.GetBoundingBox` (`self.GrindMesh`))))
  (`StaticMeshComponent.SetStaticMesh` (`self.InstancedStaticMesh`) (`self.GrindMesh`))
  (bind _output_get (set `self.Spacing` (+ (.x (- _max _min)) (`self.Offset`))))
  (bind _output_get_2 (set `local.Number of Instances` (`KismetMathLibrary.FFloor` (/ (`SplineComponent.GetSplineLength` (`self.GrindSpline`)) _output_get))))
  (for _index (range (+ _output_get_2 1))
    (bind _returnvalue (`self.GetLocationAtIndex` _index))
    (`InstancedStaticMeshComponent.AddInstance` (`self.InstancedStaticMesh`) (`KismetMathLibrary.MakeTransform` _returnvalue (`KismetMathLibrary.MakeRotFromX` (- (`self.GetLocationAtIndex` (+ _index 1)) _returnvalue))) false)))